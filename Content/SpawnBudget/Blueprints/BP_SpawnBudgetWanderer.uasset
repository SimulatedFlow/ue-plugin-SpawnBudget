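; BP_SpawnBudgetWanderer is an actor that circles the world origin on an elliptical path at a fixed height while running.
; Tick advances an angle at a degrees-per-second rate and derives the position from cosine and sine scaled by separate X and Y radii.
; It teleports there with yaw offset 90 degrees from the angle, roughly facing along the path.
; ToggleRun flips the Running flag that gates this movement.
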(event EventBeginPlay)

(event Collision|EventActorBeginOverlap
  (params (OtherActor :type Actor%20Object%20Reference)))

(event EventTick
  (params (DeltaSeconds :type Float%20%28single-precision%29))
  (if (Variables|Default|GetbRunning)
    (Variables|Default|SetAngle (+ (Variables|Default|GetAngle) (* DeltaSeconds (Variables|Default|GetDegreesPerSecond))))
    (Transformation|SetActorLocationAndRotation self (Math|Vector|MakeVector (* (Variables|Default|GetRadiusX) (Math|Trig|Cos(Degrees) (+ (Variables|Default|GetAngle) (* DeltaSeconds (Variables|Default|GetDegreesPerSecond))))) (* (Variables|Default|GetRadiusY) (Math|Trig|Sin(Degrees) (+ (Variables|Default|GetAngle) (* DeltaSeconds (Variables|Default|GetDegreesPerSecond))))) (Variables|Default|GetCenterZ)) (Math|Rotator|MakeRotator 0.0 0.0 (+ (+ (Variables|Default|GetAngle) (* DeltaSeconds (Variables|Default|GetDegreesPerSecond))) (Math|Float|MakeLiteralFloat 9e+01))) false true)))

(fn ConstructionScript)

(fn ToggleRun
  (Variables|Default|SetbRunning (not (Variables|Default|GetbRunning))))